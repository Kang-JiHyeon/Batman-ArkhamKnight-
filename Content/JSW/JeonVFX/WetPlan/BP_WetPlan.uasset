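; Wet-surface VFX actor that animates the WaterAmount of a MI_WetPlan dynamic material on its Cube, starting dry at zero.
; WetPlanButton, noted as triggered from the third-person character, flip-flops the YetStart flag on each call.
; Tick plays or reverses the StartWet timeline from that flag, and the timeline's curve drives WaterAmount for an eased transition.
; A clamped increment/decrement alternative without the timeline remains unconnected.
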(event `self.ReceiveBeginPlay`
  ;[1 1 1] 시작할때 머테리얼의 WaterAmount값을 0으로 하겠다.
  (bind _returnvalue (`PrimitiveComponent.CreateDynamicMaterialInstance` (`self.Cube`) 0 "/Game/JSW/JeonVFX/WetPlan/MI_WetPlan.MI_WetPlan" "None"))
  (`MaterialInstanceDynamic.SetScalarParameterValue` _returnvalue "WaterAmount" 0.0))

(event `self.ReceiveTick`
  (params (DeltaSeconds :type "Float (single-precision)"))
  ;[1 1 1] 버튼이 on//off가 되면 WaterAmount의 값을 조정하겠다.
  (if (`self.yetStart`)
    (bind (_direction _startwet) (`Timeline|StartWet` :`NewTime` DeltaSeconds :!label _label)
      (:`Update`
        (bind _output_get (set `self.waterAmount` _startwet))
        (`MaterialInstanceDynamic.SetScalarParameterValue` (stale `self.ReceiveBeginPlay` _returnvalue) "WaterAmount" _output_get)))
    (else
      (goto _label :!via `Reverse`))))

(event `WetPlanButton`
  ;[1 1 1] 버튼을 눌렀냐 안눌렀냐(이거 컨트롤은 써드퍼스널에서함)
  (`/Engine/EditorBlueprintResources/StandardMacros.FlipFlop`
    (:`A`
      (set `self.yetStart` true))
    (:`B`
      (set `self.yetStart` false))))

(fn `UserConstructionScript`)