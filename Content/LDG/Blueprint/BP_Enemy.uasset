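; BP_Enemy is an enemy actor that travels along a spline path from start to end.
; On BeginPlay it finds a BP_EnemySpline actor in the level through GetActorOfClass and calls Move.
; Move plays the TraceSpline timeline at a rate of 1 / TimeToComplete, mapping its Trace value to distance along the spline.
; Each update sets the actor's world location and rotation from that point on the spline.
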(event `self.ReceiveBeginPlay`
  (bind _returnvalue (`GameplayStatics.GetActorOfClass` "/Game/LDG/Blueprint/BP_EnemySpline.BP_EnemySpline_C"))
  (set `self.SplinePath` _returnvalue)
  (`self.Move`))

(event `Move`
  (bind _returnvalue (`self.GetComponentByClass` (`self.SplinePath`) "/Script/Engine.SplineComponent"))
  (`TimelineComponent.SetPlayRate` (`self.TraceSpline`) (/ 1.0 (`self.TimeToComplete`)))
  (bind (_direction _trace) (`Timeline|TraceSpline`)
    (:`Update`
      (bind _returnvalue_2 (`KismetMathLibrary.Lerp` 0.0 (`SplineComponent.GetSplineLength` (`self.GetComponentByClass` (`self.SplinePath`) "/Script/Engine.SplineComponent")) _trace))
      (`self.K2_SetActorTransform` (`KismetMathLibrary.MakeTransform` (`SplineComponent.GetLocationAtDistanceAlongSpline` _returnvalue _returnvalue_2 "World") (`SplineComponent.GetRotationAtDistanceAlongSpline` _returnvalue _returnvalue_2 "World"))))))

(fn `UserConstructionScript`)