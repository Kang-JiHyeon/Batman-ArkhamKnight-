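; Game mode for a Batmobile chase that drives the chase audio from the state of the enemy vehicle.
; On BeginPlay it finds a BP_VehicleEnemy actor, stores it and plays the InChase 2D sound.
; Tick polls that enemy's IsAttackAble flag and plays ChaseComplete whenever it is false, with no one-shot guard, so the sound starts again every frame.
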(event `self.ReceiveBeginPlay`
  (`parent.ReceiveBeginPlay`)
  (bind _returnvalue (`GameplayStatics.GetActorOfClass` "/Game/LDG/Blueprint/BP_VehicleEnemy.BP_VehicleEnemy_C"))
  (`GameplayStatics.PlaySound2D` "/Game/LDG/Assets/FX/SFX/InChase.InChase" 1.0 1.0 0.0 null null))

(event `self.ReceiveTick`
  (params (DeltaSeconds :type "Float (single-precision)"))
  (`parent.ReceiveTick` DeltaSeconds)
  (if (not (`VehicleEnemy.bIsAttackAble` (stale `self.ReceiveBeginPlay` _returnvalue)))
    (`GameplayStatics.PlaySound2D` "/Game/LDG/Assets/FX/SFX/ChaseComplete.ChaseComplete" 1.0 1.0 0.0 null null)))

(fn `UserConstructionScript`
  (`parent.UserConstructionScript`))