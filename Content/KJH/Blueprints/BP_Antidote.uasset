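; BP_Antidote is an antidote actor that toggles UI as the player approaches, with no pickup logic in this graph.
; On BeginPlay it creates and shows the KJH boss map mission widget.
; While Active, a PlayerCharacter overlap stores the player, hides the mission widget and shows the actor's own Widget; leaving reverses this.
; The Tab key only prints a debug string, noted as belonging on the player.
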(event `self.ReceiveBeginPlay`
  (bind _returnvalue (`|CreateWidget` "/Game/KJH/UI/WBP_KJHBossMapMission.WBP_KJHBossMapMission_C"))
  (bind _output_get (set `self.MissionWidget` _returnvalue))
  (`UserWidget.AddToViewport` _output_get 0)
  (`Widget.SetVisibility` _output_get "Visible"))

(event `self.ReceiveActorBeginOverlap`
  (params (OtherActor :type "Actor Object Reference"))
  (if (`self.bActive`)
    (bind _asplayer_character (cast `PlayerCharacter` OtherActor))
    (set `self.Player` _asplayer_character)
    (`/Engine/EditorBlueprintResources/StandardMacros.IsValid` _asplayer_character
      (:`Is Valid`
        (`Widget.SetVisibility` (`self.MissionWidget`) "Hidden")
        (`SceneComponent.SetVisibility` (`self.Widget`) true false)))))

(event `self.ReceiveActorEndOverlap`
  (params (OtherActor :type "Actor Object Reference"))
  (if (== OtherActor (`self.Player`))
    (set `self.Player` null)
    (`Widget.SetVisibility` (`self.MissionWidget`) "Visible")
    (`SceneComponent.SetVisibility` (`self.Widget`) false false)))

(event `Key|Tab`
  (params (Key :type "Key Structure"))
  ;[1 1 1] 플레이어가ㅣ 해야함
  (:`Pressed`
    (`KismetSystemLibrary.PrintString` "Hello")))

(fn `UserConstructionScript`)