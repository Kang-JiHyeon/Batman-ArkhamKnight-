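; BP_TestEnemy is a test enemy that moves back and forth along its forward axis.
; Tick offsets the actor's location along its forward vector by Speed and delta time, without sweeping for collision.
; A looping timer started on BeginPlay calls OnChangedDirection every few seconds, which negates Speed to reverse travel without rotating the actor.
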(event `self.ReceiveBeginPlay`
  (`KismetSystemLibrary.K2_SetTimer` null "OnChangedDirection" 3.0 true))

(event `self.ReceiveTick`
  (params (DeltaSeconds :type "Float (single-precision)"))
  (`self.K2_SetActorLocation` (+ (`self.K2_GetActorLocation`) (* DeltaSeconds (`self.Speed`) (`self.GetActorForwardVector`)))))

(fn `OnChangedDirection`
  (set `self.Speed` (* (`self.Speed`) -1.0)))

(fn `UserConstructionScript`)