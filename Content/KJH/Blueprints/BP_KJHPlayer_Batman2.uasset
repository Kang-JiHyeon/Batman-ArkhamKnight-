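; Batman player character Blueprint, apparently a testbed for a motion-warped attack on a boss, left unwired.
; The boss attack input event is empty; the chain that would call TestMotionWarping and play the attack montage is disconnected.
; TestMotionWarping only reads boss and player locations.
; Its disconnected warp-target update would place "AttactPoint" a short distance from the boss on the player's side, facing the boss.
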(event `EnhancedInput|/Game/KJH/Input/InputAction/IA_KJHBossAttack`
  (params (ActionValue :type Boolean) (ElapsedSeconds :type "Float (double-precision)") (TriggeredSeconds :type "Float (double-precision)") (InputAction :type "InputAction Object Reference" :default "/Game/KJH/Input/InputAction/IA_KJHBossAttack.IA_KJHBossAttack")))

(fn `Test_MotionWarping`
  (set `self.TargetLoc` (`self.K2_GetActorLocation` (`self.TargetBoss`)))
  (set `self.PlayerLoc` (`self.K2_GetActorLocation`)))

(fn `UserConstructionScript`)