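; BP_AntidoteDetector is an overlap trigger that makes itself the player's antidote interaction target.
; BeginPlay reuses an existing boss map mission widget or creates one.
; While active, player overlap registers it with the player's PlayerAntidoteDetector component, hides the mission widget and shows the Tab interaction prompt.
; When that player leaves, it clears the target and swaps the widgets back.
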(event `self.ReceiveBeginPlay`
  (bind _foundwidgets (`WidgetBlueprintLibrary.GetAllWidgetsOfClass` "/Game/KJH/UI/WBP_KJHBossMapMission.WBP_KJHBossMapMission_C"))
  (if (<= (`KismetArrayLibrary.Array_Length` _foundwidgets) 0)
    (bind _returnvalue (`|CreateWidget` "/Game/KJH/UI/WBP_KJHBossMapMission.WBP_KJHBossMapMission_C"))
    (bind _output_get (set `self.MissionWidget` _returnvalue))
    (`UserWidget.AddToViewport` _output_get 0)
    (`Widget.SetVisibility` _output_get "Visible")
    (else
      (set `self.MissionWidget` (`|GetArrayItem` _foundwidgets)))))

(event `self.ReceiveActorBeginOverlap`
  (params (OtherActor :type "Actor Object Reference"))
  (if (`self.bActive`)
    (bind _asplayer_character (cast `PlayerCharacter` OtherActor))
    (bind _output_get (set `self.Player` _asplayer_character))
    (`/Engine/EditorBlueprintResources/StandardMacros.IsValid` _output_get
      (:`Is Valid`
        (`self.SetPlayerTargetAntidote` (`self.Player`) self)
        (`self.ShowInteractionGuide` true)))))

(event `self.ReceiveActorEndOverlap`
  (params (OtherActor :type "Actor Object Reference"))
  (if (== OtherActor (`self.Player`))
    (`self.SetPlayerTargetAntidote` (`self.Player`))
    (set `self.Player` null)
    (`self.ShowInteractionGuide` false)))

(fn `SetPlayerTargetAntidote`
  (params (Player :type "PlayerCharacter Object Reference") (TargetActor :type "Actor Object Reference"))
  (bind _returnvalue (`self.GetComponentByClass` Player "/Script/Batman_ArkhamKnight.PlayerAntidoteDetector"))
  (`/Engine/EditorBlueprintResources/StandardMacros.IsValid` _returnvalue
    (:`Is Valid`
      (`PlayerAntidoteDetector.SetTargetAntidote` _returnvalue TargetActor))))

(fn `ShowInteractionGuide`
  (params (bShowInteractonGuide :type Boolean))
  (if bShowInteractonGuide
    (`Widget.SetVisibility` (`self.MissionWidget`) "Hidden")
    (`SceneComponent.SetVisibility` (`self.TabInteractionWidget`) true false)
    (else
      (`Widget.SetVisibility` (`self.MissionWidget`) "Visible")
      (`SceneComponent.SetVisibility` (`self.TabInteractionWidget`) false false))))

(fn `UserConstructionScript`)